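; BP_Projectile is a physics projectile actor, described in its comments as a cannonball, with callable functions and no active event logic.
; Launch applies a velocity-change impulse to its static mesh along the actor's forward vector.
; Explosion spawns an actor, with no class shown, just ahead of the player pawn rather than at the projectile.
; PrintYourName prints the actor's display name.
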(event EventBeginPlay)

(event Collision|EventActorBeginOverlap
  (params (OtherActor :type Actor%20Object%20Reference)))

(event EventTick
  (params (DeltaSeconds :type Float%20%28single-precision%29)))

(fn ConstructionScript)

(fn PrintYourName
  (Development|PrintString (Utilities|GetDisplayName self)))

(fn Launch
  (Physics|AddImpulse (Variables|/Script/Engine.StaticMeshActor|GetStaticMeshComponent self) (* (Transformation|GetActorForwardVector) 6e+03) "None" true) ; We have to get the control rotation from the player pawn enable to have the spaw of the cannon balls to be spawned where we look at.
)

(fn Explosion
  (bind _returnvalue (Game|Player|GetPlayerPawn 0))
  (Game|SpawnActorfromClass "/Game/StarterContent/Blueprints/Blueprint_Effect_Explosion.Blueprint_Effect_Explosion_C" (Math|Conversions|ToTransform(Vector) (+ (Transformation|GetActorLocation _returnvalue) (Transformation|GetActorForwardVector _returnvalue))) "Undefined" 0 0))